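; A child of the Mordhau player character that serves as a debug tool for dumping the game's color table data.
; Pressing the Divide key loops through the first eight color tables in the Mordhau singleton, formatting each table name and every entry's class name and color.
; Each line is sent as a chat message through the player controller and collected in an array, which is saved to a ColorDataDump text file, then cleared.
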(event `Key|Divide`
  (params (Key :type "Key Structure"))
  (bind _newvar_1 (`self.NewVar_1`))
  (:`Pressed`
    (for _index (range 8)
      (bind (_tablename _entries) (break `MordhauColorItemTable` (`|GetArrayItem` (`MordhauSingleton.ColorTables` (`MordhauUtilityLibrary.GetMordhauSingleton`)) _index)))
      (bind _returnvalue (`KismetStringLibrary.Concat_StrStr` "ID:    " (`KismetStringLibrary.Conv_IntToString` _index) "      Table Name:     " (`KismetTextLibrary.Conv_TextToString` _tablename)))
      (`self.NewFunction_0` _returnvalue)
      (bind _returnvalue_2 (`KismetArrayLibrary.Array_Add` _newvar_1 _returnvalue))
      (`KismetArrayLibrary.Array_Set` _newvar_1 _returnvalue_2 _returnvalue true)
      (for (_array_element _array_index) _entries
        (bind _returnvalue_3 (`KismetStringLibrary.Concat_StrStr` "ID:   " (`KismetStringLibrary.Conv_IntToString` _array_index) "     BP_Name:     " (`KismetSystemLibrary.GetClassDisplayName` _array_element) "    Color:    " (`KismetStringLibrary.Conv_ColorToString` (`KismetMathLibrary.Conv_ColorToLinearColor` (`KismetMathLibrary.LinearColor_ToRGBE` (defaults `Object` _array_element))))))
        (`self.NewFunction_0` _returnvalue_3)
        (bind _returnvalue_4 (`KismetArrayLibrary.Array_Add` _newvar_1 _returnvalue_3))
        (`KismetArrayLibrary.Array_Set` _newvar_1 _returnvalue_4 _returnvalue_3 true)))
    (`MordhauUtilityLibrary.SaveStringArrayToFile` "ColorDataDump" _newvar_1)
    (`KismetSystemLibrary.Delay` 1.0)
    (`KismetArrayLibrary.Array_Clear` _newvar_1)))

(fn `NewFunction_0`
  (params (NewParam :type String))
  (bind _asbp_mordhau_player_controller (cast `/Game/Mordhau/Blueprints/BP_MordhauPlayerController` (`GameplayStatics.GetPlayerController` 0)))
  (`/Game/Mordhau/Blueprints/BP_MordhauPlayerController.RequestChatMessage` _asbp_mordhau_player_controller NewParam false))

(fn `UserConstructionScript`
  (`parent.UserConstructionScript`))